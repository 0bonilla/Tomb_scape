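; BP_ButtonPuzzle1 is a pressable puzzle button that animates in and back out; no puzzle logic is in this graph.
; Pressed plays a move sound and runs the Push timeline, sliding the mesh slightly along relative Y.
; On finish, a Loop flag alternates between replaying the sound while reversing and clearing IsPressed, which blocks re-presses during animation.
; The sound location uses the mesh's relative, not world, location.
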(event Custom|Pressed
  (if (not (Variables|Default|GetIsPressed))
    (Audio|PlaySoundatLocation "/Game/Assets/Sounds/PreassurePlateMove.PreassurePlateMove" (Variables|/Script/Engine.SceneComponent|GetRelativeLocation (Variables|Default|GetAssets2_LocationObject3)) "0, 0, 0" 1.0 1.0 0.0 0 0 0 0)
    (bind _push (Timeline|Push Play)
      (:Update
        (Transformation|SetRelativeLocation (Variables|Default|GetAssets2_LocationObject3) (Math|Vector|MakeVector 0.0 (Math|Float|Lerp 0.0 -1.5 _push) 0.0) false false)
        (Variables|Default|SetIsPressed true))
      (:Finished
        (if (Variables|Default|GetLoop)
          (Variables|Default|SetLoop false)
          (Audio|PlaySoundatLocation "/Game/Assets/Sounds/PreassurePlateMove.PreassurePlateMove" (Variables|/Script/Engine.SceneComponent|GetRelativeLocation (Variables|Default|GetAssets2_LocationObject3)) "0, 0, 0" 1.0 1.0 0.0 0 0 0 0)
          (Timeline|Push Reverse)
          (else
            (Variables|Default|SetLoop true)
            (Variables|Default|SetIsPressed false)))))))

(fn ConstructionScript)