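; BP_Puzzle2 is a puzzle counter that shows an integer on a TextRender component.
; BeginPlay displays the initial Contador value.
; The Increase event adds one to Contador, resets it to zero once it exceeds eight, then updates the text from the increment's output.
; No caller of Increase or solution check appears in this Blueprint.
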(event Custom|Increase
  (bind _result (Math|Integer|IncrementInt (Variables|Default|GetContador))
    (:%20%20
      (if (> _result 8)
        (Variables|Default|SetContador 0))
      (Rendering|Components|TextRender|SetText (Variables|Default|GetTextRender) (Utilities|Text|ToText(Integer) _result)))))

(event EventBeginPlay
  (Rendering|Components|TextRender|SetText (Variables|Default|GetTextRender) (Utilities|Text|ToText(Integer) (Variables|Default|GetContador))))

(fn ConstructionScript)