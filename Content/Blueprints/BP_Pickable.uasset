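; Pickable physics item, with a Hammer component, that the player can pick up and hold through an interaction event.
; Interacting stores the player and, if their hands are empty, snaps the item to their ItemGrip, turns off physics and collision, and registers it as CurrentHeldItem.
; DropItem detaches it, places it just in front of the camera and restores physics and collision, without clearing CurrentHeldItem.
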(event EventBeginPlay)

(event Collision|EventActorBeginOverlap
  (params (OtherActor :type Actor%20Object%20Reference)))

(event EventTick
  (params (DeltaSeconds :type Float%20%28single-precision%29)))

(event EventLookat
  (params (PlayerCharacter :type BP%20First%20Person%20Character%20Object%20Reference)))

(event EventInteractwith
  (params (PlayerCharacter :type BP%20First%20Person%20Character%20Object%20Reference))
  (bind _output_get (Variables|Default|SetPlayer PlayerCharacter))
  (Variables|/Game/FirstPerson/Blueprints/BP_FirstPersonCharacter.BP_FirstPersonCharacter_C|GetCurrentHeldItem _output_get
    (:then)
    (:else
      (CallFunction|PickUpItem))))

(fn ConstructionScript)

(fn PickUpItem
  (bind _hammer (Variables|Default|GetHammer))
  (Transformation|AttachComponentToComponent (Variables|/Game/FirstPerson/Blueprints/BP_FirstPersonCharacter.BP_FirstPersonCharacter_C|GetItemGrip (Variables|Default|GetPlayer)) "None" "SnapToTarget" "SnapToTarget" "KeepRelative" true)
  (Physics|SetSimulatePhysics _hammer false)
  (Collision|SetCollisionEnabled _hammer "NoCollision")
  (Variables|/Game/FirstPerson/Blueprints/BP_FirstPersonCharacter.BP_FirstPersonCharacter_C|SetCurrentHeldItem (Variables|Default|GetPlayer) self))

(fn DropItem
  (bind _returnvalue (Game|GetPlayerCameraManager 0))
  (bind _hammer (Variables|Default|GetHammer))
  (Transformation|DetachFromActor "KeepWorld" "KeepWorld" "KeepWorld")
  (Transformation|SetActorLocation (+ (Camera|GetCameraLocation _returnvalue) (* (Math|Vector|GetForwardVector (Camera|GetCameraRotation _returnvalue)) 5e+01)) false false)
  (Physics|SetSimulatePhysics _hammer true)
  (Collision|SetCollisionEnabled _hammer "QueryAndPhysics"))