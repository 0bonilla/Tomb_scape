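; BP_Chest is a chest that starts hidden and holds a key the player picks up to set PassToThird on the first-person character.
; Custom events toggle its visibility and collision, with ShowAfterAnimation available to reveal it after an animation.
; The Box overlap shows an interact prompt widget and enables input only while the player is inside.
; Pressing E then hides the key mesh and sets the flag.
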(event OnComponentBeginOverlap(Box)
  (params (OverlappedComponent :type Primitive%20Component%20Object%20Reference) (OtherActor :type Actor%20Object%20Reference) (OtherComp :type Primitive%20Component%20Object%20Reference) (OtherBodyIndex :type Integer) (bFromSweep :type Boolean) (SweepResult :type Hit%20Result%20Structure%20%28by%20ref%29))
  (if (== OtherActor (Variables|Default|GetPlayerRef))
    (UserInterface|Viewport|AddtoViewport (Variables|Default|GetMessage) 0)
    (Input|EnableInput (Game|GetPlayerController 0))
    (Variables|Default|SetCanPickUp true)))

(event OnComponentEndOverlap(Box)
  (params (OverlappedComponent :type Primitive%20Component%20Object%20Reference) (OtherActor :type Actor%20Object%20Reference) (OtherComp :type Primitive%20Component%20Object%20Reference) (OtherBodyIndex :type Integer))
  (if (== (Variables|Default|GetPlayerRef) OtherActor)
    (Widget|RemovefromParent (Variables|Default|GetMessage))
    (Input|DisableInput (Game|GetPlayerController 0))
    (Variables|Default|SetCanPickUp false)))

(event Custom|HideBeforeAnimation
  (Rendering|SetVisibility (Variables|Default|GetDefaultSceneRoot) false true)
  (Collision|SetCollisionEnabled (Variables|Default|GetChestTop) "NoCollision")
  (Collision|SetCollisionEnabled (Variables|Default|GetChestBase) "NoCollision")
  (Collision|SetCollisionEnabled (Variables|Default|GetBox) "NoCollision"))

(event Custom|ShowAfterAnimation
  (Rendering|SetVisibility (Variables|Default|GetDefaultSceneRoot) true true)
  (Collision|SetCollisionEnabled (Variables|Default|GetChestTop) "QueryAndPhysics")
  (Collision|SetCollisionEnabled (Variables|Default|GetChestBase) "QueryAndPhysics")
  (Collision|SetCollisionEnabled (Variables|Default|GetBox) "QueryAndPhysics"))

(event EventBeginPlay
  (CallFunction|HideBeforeAnimation)
  (bind _asbp_first_person_character (Utilities|Casting|CastToBP_FirstPersonCharacter (Game|GetPlayerCharacter 0)))
  (Variables|Default|SetPlayerRef _asbp_first_person_character)
  (bind _returnvalue (UserInterface|CreateWidget "/Game/Interfaces/WB_InteractPrompt.WB_InteractPrompt_C"))
  (Variables|Default|SetMessage _returnvalue))

(event Input|KeyboardEvents|E
  (params (Key :type Key%20Structure :default "None"))
  (:Pressed
    (if (Variables|Default|GetCanPickUp)
      (Rendering|SetVisibility (Variables|Default|GetKey) false false)
      (Variables|/Game/FirstPerson/Blueprints/BP_FirstPersonCharacter.BP_FirstPersonCharacter_C|SetPassToThird (Variables|Default|GetPlayerRef) true))))

(fn ConstructionScript)