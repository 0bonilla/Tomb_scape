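; BP_DecitionDoorKey is a key pickup that grants the first-person player the Decition key.
; Overlapping its Box shows an interact prompt widget and enables actor input; leaving reverses both.
; Pressing E in range plays a sound, sets HasDecitionKey on the player and destroys the Box and Llave components.
; A timeline then lerps the Pilar component downward.
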(event OnComponentBeginOverlap(Box)
  (params (OverlappedComponent :type Primitive%20Component%20Object%20Reference) (OtherActor :type Actor%20Object%20Reference) (OtherComp :type Primitive%20Component%20Object%20Reference) (OtherBodyIndex :type Integer) (bFromSweep :type Boolean) (SweepResult :type Hit%20Result%20Structure%20%28by%20ref%29))
  (if (== OtherActor (Variables|Default|GetPlayerRef))
    (UserInterface|Viewport|AddtoViewport (Variables|Default|GetMessage) 0)
    (Input|EnableInput (Game|GetPlayerController 0))
    (Variables|Default|SetPlayerCanCollectKey true)))

(event OnComponentEndOverlap(Box)
  (params (OverlappedComponent :type Primitive%20Component%20Object%20Reference) (OtherActor :type Actor%20Object%20Reference) (OtherComp :type Primitive%20Component%20Object%20Reference) (OtherBodyIndex :type Integer))
  (if (== (Variables|Default|GetPlayerRef) OtherActor)
    (Widget|RemovefromParent (Variables|Default|GetMessage))
    (Input|DisableInput (Game|GetPlayerController 0))
    (Variables|Default|SetPlayerCanCollectKey false)))

(event EventBeginPlay
  (bind _asbp_first_person_character (Utilities|Casting|CastToBP_FirstPersonCharacter (Game|GetPlayerCharacter 0)))
  (Variables|Default|SetPlayerRef _asbp_first_person_character)
  (bind _returnvalue (UserInterface|CreateWidget "/Game/Interfaces/WB_InteractPrompt.WB_InteractPrompt_C"))
  (Variables|Default|SetMessage _returnvalue))

(event Input|KeyboardEvents|E
  (params (Key :type Key%20Structure :default "None"))
  (:Pressed
    (if (Variables|Default|GetPlayerCanCollectKey)
      (Audio|PlaySound2D "/Game/Assets/Sounds/GrabKey.GrabKey" 1.0 1.0 0.0 0 0)
      (Variables|/Game/FirstPerson/Blueprints/BP_FirstPersonCharacter.BP_FirstPersonCharacter_C|SetHasDecitionKey (Variables|Default|GetPlayerRef) true)
      (Components|DestroyComponent (Variables|Default|GetLlave2))
      (Components|DestroyComponent (Variables|Default|GetBox))
      (Components|DestroyComponent (Variables|Default|GetLlave3))
      (bind _pilardown (Timeline|PilarMovement Play)
        (:Update
          (Transformation|SetRelativeLocation (Variables|Default|GetPilar) (Math|Vector|MakeVector 0.0 0.0 (Math|Float|Lerp -85.0 -1.8e+02 _pilardown)) false false))))))

(fn ConstructionScript)