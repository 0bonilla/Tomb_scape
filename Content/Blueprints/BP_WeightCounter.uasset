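; BP_WeightCounter is a Blueprint that displays the total weight on a scale through a text render component.
; It shows the stored total as integer text on BeginPlay.
; Increase and Decrease events behave identically, replacing the stored total with the value passed in and refreshing the text, so the caller supplies the new total rather than a difference.
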(event Custom|Decrease
  (params (Weight :type Integer))
  (bind _output_get (Variables|Default|SetTotalWeightOnScale Weight))
  (Rendering|Components|TextRender|SetText (Variables|Default|GetTextRender) (Utilities|Text|ToText(Integer) _output_get)))

(event Custom|Increase
  (params (NewWeigh :type Integer))
  (bind _output_get (Variables|Default|SetTotalWeightOnScale NewWeigh))
  (Rendering|Components|TextRender|SetText (Variables|Default|GetTextRender) (Utilities|Text|ToText(Integer) _output_get)))

(event EventBeginPlay
  (Rendering|Components|TextRender|SetText (Variables|Default|GetTextRender) (Utilities|Text|ToText(Integer) (Variables|Default|GetTotalWeightOnScale))))

(fn ConstructionScript)