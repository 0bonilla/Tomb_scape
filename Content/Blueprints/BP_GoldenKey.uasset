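; BP_GoldenKey is a collectible key for the last puzzle, picked up with E while the player stands in its sphere.
; Overlap shows or hides an interact prompt widget and toggles the key's input.
; Pickup increments the player's KeysLastPuzzle counter, plays a sound and destroys the key.
; The third key also finds BP_DoorHammer, calls DestroyLock on it and plays a door sound.
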(event OnComponentBeginOverlap(Sphere)
  (params (OverlappedComponent :type Primitive%20Component%20Object%20Reference) (OtherActor :type Actor%20Object%20Reference) (OtherComp :type Primitive%20Component%20Object%20Reference) (OtherBodyIndex :type Integer) (bFromSweep :type Boolean) (SweepResult :type Hit%20Result%20Structure%20%28by%20ref%29))
  (if (== OtherActor (Variables|Default|GetPlayerRef))
    (UserInterface|Viewport|AddtoViewport (Variables|Default|GetMessage) 0)
    (Input|EnableInput (Game|GetPlayerController 0))
    (Variables|Default|SetCanPickUp true)))

(event OnComponentEndOverlap(Sphere)
  (params (OverlappedComponent :type Primitive%20Component%20Object%20Reference) (OtherActor :type Actor%20Object%20Reference) (OtherComp :type Primitive%20Component%20Object%20Reference) (OtherBodyIndex :type Integer))
  (if (== (Variables|Default|GetPlayerRef) OtherActor)
    (Widget|RemovefromParent (Variables|Default|GetMessage))
    (Input|DisableInput (Game|GetPlayerController 0))
    (Variables|Default|SetCanPickUp false)))

(event EventBeginPlay
  (bind _asbp_first_person_character (Utilities|Casting|CastToBP_FirstPersonCharacter (Game|GetPlayerCharacter 0)))
  (Variables|Default|SetPlayerRef _asbp_first_person_character)
  (bind _returnvalue (UserInterface|CreateWidget "/Game/Interfaces/WB_InteractPrompt.WB_InteractPrompt_C"))
  (Variables|Default|SetMessage _returnvalue))

(event Input|KeyboardEvents|E
  (params (Key :type Key%20Structure :default "None"))
  (bind _playerref (Variables|Default|GetPlayerRef))
  (:Pressed
    (if (Variables|Default|GetCanPickUp)
      (bind _result (Math|Integer|IncrementInt (Variables|/Game/FirstPerson/Blueprints/BP_FirstPersonCharacter.BP_FirstPersonCharacter_C|GetKeysLastPuzzle _playerref))
        (:%20%20
          (bind _output_get (Variables|/Game/FirstPerson/Blueprints/BP_FirstPersonCharacter.BP_FirstPersonCharacter_C|SetKeysLastPuzzle _playerref _result))
          (Utilities|FlowControl|Sequence
            (:then_0
              (Audio|PlaySound2D "/Game/Assets/Sounds/GrabKey.GrabKey" 1.0 1.0 0.0 0 0)
              (Actor|DestroyActor))
            (:then_1
              (if (== _output_get 3)
                (bind _returnvalue (Actor|GetActorOfClass "/Game/Blueprints/DoorBlueprint/BP_DoorHammer.BP_DoorHammer_C"))
                (Default|DestroyLock _returnvalue)
                (Audio|PlaySound2D "/Game/Assets/Sounds/DoorLocked.DoorLocked" 1.0 1.0 0.0 0 0)))))))))

(fn ConstructionScript)