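; Pressure plate that reacts only to the player character, reporting a correct or wrong press depending on IsCorrect.
; Overlap begin and end play a move sound and run the ButtonMovement timeline forward or in reverse to lower or raise the button.
; When the timeline finishes fully pressed, it calls PreassurePressed once for a correct plate, guarded by WasPressed, or WrongPreassurePlate on every press of a wrong one.
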(event OnComponentBeginOverlap(Collider)
  (params (OverlappedComponent :type Primitive%20Component%20Object%20Reference) (OtherActor :type Actor%20Object%20Reference) (OtherComp :type Primitive%20Component%20Object%20Reference) (OtherBodyIndex :type Integer) (bFromSweep :type Boolean) (SweepResult :type Hit%20Result%20Structure%20%28by%20ref%29))
  ;[1 1 1] Button Animation
  (if (== OtherActor (Variables|Default|GetPlayerRef))
    (Utilities|FlowControl|Sequence
      (:then_0
        (bind _buttonmovement (Timeline|ButtonMovement Play)
          (:Update
            (Transformation|SetRelativeLocation (Variables|Default|GetButton) (Math|Vector|MakeVector 0.0 0.0 (Math|Float|Lerp 0.0 -1e+01 _buttonmovement)) false false))
          (:Finished
            ;[1 1 1] Llamado al Lvl BP
            (if (== (Math|Float|Lerp 0.0 -1e+01 _buttonmovement) -1e+01)
              (if (Variables|Default|GetIsCorrect)
                (if (Variables|Default|GetwasPressed)
                  (Development|PrintString "Already Pressed")
                  (else
                    (Variables|Default|SetwasPressed true)
                    (Default|CallPreassurePressed)))
                (else
                  (Default|CallWrongPreassurePlate)))))))
      (:then_1
        (Audio|PlaySoundatLocation "/Game/Assets/Sounds/PreassurePlateMove.PreassurePlateMove" (Variables|/Script/Engine.SceneComponent|GetRelativeLocation (Variables|Default|GetButton)) "0, 0, 0" 1.0 1.0 0.0 0 0 0 0)))))

(event OnComponentEndOverlap(Collider)
  (params (OverlappedComponent :type Primitive%20Component%20Object%20Reference) (OtherActor :type Actor%20Object%20Reference) (OtherComp :type Primitive%20Component%20Object%20Reference) (OtherBodyIndex :type Integer))
  ;[1 1 1] Button Animation
  (if (== (Variables|Default|GetPlayerRef) OtherActor)
    (Utilities|FlowControl|Sequence
      (:then_0
        (bind _buttonmovement (Timeline|ButtonMovement ReverseFromEnd)
          (:Update
            (Transformation|SetRelativeLocation (Variables|Default|GetButton) (Math|Vector|MakeVector 0.0 0.0 (Math|Float|Lerp 0.0 -1e+01 _buttonmovement)) false false))
          (:Finished
            ;[1 1 1] Llamado al Lvl BP
            (if (== (Math|Float|Lerp 0.0 -1e+01 _buttonmovement) -1e+01)
              (if (Variables|Default|GetIsCorrect)
                (if (Variables|Default|GetwasPressed)
                  (Development|PrintString "Already Pressed")
                  (else
                    (Variables|Default|SetwasPressed true)
                    (Default|CallPreassurePressed)))
                (else
                  (Default|CallWrongPreassurePlate)))))))
      (:then_1
        (Audio|PlaySoundatLocation "/Game/Assets/Sounds/PreassurePlateMove.PreassurePlateMove" (Variables|/Script/Engine.SceneComponent|GetRelativeLocation (Variables|Default|GetButton)) "0, 0, 0" 1.0 1.0 0.0 0 0 0 0)))))

(event EventBeginPlay
  (bind _asbp_first_person_character (Utilities|Casting|CastToBP_FirstPersonCharacter (Game|GetPlayerCharacter 0)))
  (Variables|Default|SetPlayerRef _asbp_first_person_character))

(fn ConstructionScript)