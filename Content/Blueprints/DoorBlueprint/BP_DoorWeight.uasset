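; Interactive door that swings open or closed on E, but only while its WeightPuzzle flag is true.
; A trigger box shows the interact prompt and enables input plus a gate while the player is inside.
; A FlipFlop alternates playing and reversing a yaw timeline, with an Amplitud check limiting toggles to near either end of the swing.
; Otherwise, DoorLocked plays a locked sound and a slight timeline-driven rattle.
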(event OnComponentBeginOverlap(Box)
  (params (OverlappedComponent :type Primitive%20Component%20Object%20Reference) (OtherActor :type Actor%20Object%20Reference) (OtherComp :type Primitive%20Component%20Object%20Reference) (OtherBodyIndex :type Integer) (bFromSweep :type Boolean) (SweepResult :type Hit%20Result%20Structure%20%28by%20ref%29))
  (if (== OtherActor (Variables|Default|GetPlayerRef))
    (UserInterface|Viewport|AddtoViewport (Variables|Default|GetMessage) 0)
    (Input|EnableInput (Game|GetPlayerController 0))
    (Utilities|FlowControl|Gate true) ; enters at Open
  ))

(event OnComponentEndOverlap(Box)
  (params (OverlappedComponent :type Primitive%20Component%20Object%20Reference) (OtherActor :type Actor%20Object%20Reference) (OtherComp :type Primitive%20Component%20Object%20Reference) (OtherBodyIndex :type Integer))
  (if (== (Variables|Default|GetPlayerRef) OtherActor)
    (Widget|RemovefromParent (Variables|Default|GetMessage))
    (Input|DisableInput (Game|GetPlayerController 0))
    (Utilities|FlowControl|Gate true) ; enters at Close
  ))

(event Custom|DoorLocked
  (Audio|PlaySoundatLocation "/Game/Assets/Sounds/DoorLocked.DoorLocked" (Variables|/Script/Engine.SceneComponent|GetRelativeLocation (Variables|Default|GetPuerta)) "0, 0, 0" 1.0 1.0 0.0 0 0 0 0)
  (bind _newtrack_0 (Timeline|Timeline_0 PlayFromStart)
    (:Update
      (Transformation|SetRelativeRotation (Variables|Default|GetPuerta) (Math|Rotator|MakeRotator 0.0 0.0 (Math|Float|Lerp 0.0 5.0 _newtrack_0)) false false))))

(event EventBeginPlay
  (bind _asbp_first_person_character (Utilities|Casting|CastToBP_FirstPersonCharacter (Game|GetPlayerCharacter 0)))
  (Variables|Default|SetPlayerRef _asbp_first_person_character)
  (bind _returnvalue (UserInterface|CreateWidget "/Game/Interfaces/WB_InteractPrompt.WB_InteractPrompt_C"))
  (Variables|Default|SetMessage _returnvalue))

(event Input|KeyboardEvents|E
  (params (Key :type Key%20Structure :default "None"))
  (:Pressed
    (if (Variables|Default|GetWeightPuzzle)
      (if (or (>= (Variables|Default|GetAmplitud) 119.0) (<= (Variables|Default|GetAmplitud) 1.0))
        (Utilities|FlowControl|Gate true
          (:Exit
            (Audio|PlaySoundatLocation "/Game/Assets/Sounds/MetalDoor.MetalDoor" (Variables|/Script/Engine.SceneComponent|GetRelativeLocation (Variables|Default|GetPuerta)) "0, 0, 0" 1.0 1.0 0.0 0 0 0 0)
            (Utilities|FlowControl|FlipFlop
              (:A
                (bind _newtrack_0 (Timeline|Timeline Play)
                  (:Update
                    (Variables|Default|SetAmplitud _newtrack_0)
                    (Transformation|SetRelativeRotation (Variables|Default|GetPuerta) (Math|Rotator|MakeRotator 0.0 0.0 _newtrack_0) false false))))
              (:B
                (Timeline|Timeline Reverse))))))
      (else
        (CallFunction|DoorLocked)))))

(fn ConstructionScript)