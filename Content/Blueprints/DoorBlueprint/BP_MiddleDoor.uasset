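; BP_MiddleDoor is a door actor that swings open with a metal sound when its DoorInteraction event fires.
; DoorInteraction plays the sound at the door mesh's relative location, then plays DoorTimeline forward to drive the mesh's relative yaw, with no reverse path.
; BeginPlay caches the first-person character in PlayerRef, which nothing else in these graphs reads.
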(event Custom|DoorInteraction
  (Audio|PlaySoundatLocation "/Game/Assets/Sounds/MetalDoor.MetalDoor" (Variables|/Script/Engine.SceneComponent|GetRelativeLocation (Variables|Default|GetSM_Door)) "0, 0, 0" 1.0 1.0 0.0 0 0 0 0)
  (bind _newtrack_0 (Timeline|DoorTimeline Play)
    (:Update
      (Transformation|SetRelativeRotation (Variables|Default|GetSM_Door) (Math|Rotator|MakeRotator 0.0 0.0 _newtrack_0) false false))))

(event EventBeginPlay
  (bind _asbp_first_person_character (Utilities|Casting|CastToBP_FirstPersonCharacter (Game|GetPlayerCharacter 0)))
  (Variables|Default|SetPlayerRef _asbp_first_person_character))

(fn ConstructionScript)