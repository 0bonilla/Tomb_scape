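; Two-scale weight puzzle with a digital weight readout on each pillar.
; Overlap boxes add or subtract the Weigh value of BP_Weight1 actors and push each total to a BP_WeightCounter child actor.
; When the totals match, timelines move both pillars vertically, then a sound plays and BP_DoorWeight's WeightPuzzle flag is set.
; CheckResult runs only on overlap changes, and nothing reverses a solved state.
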(event OnComponentEndOverlap(Box)
  (params (OverlappedComponent :type Primitive%20Component%20Object%20Reference) (OtherActor :type Actor%20Object%20Reference) (OtherComp :type Primitive%20Component%20Object%20Reference) (OtherBodyIndex :type Integer))
  ;[1 1 1] Scale 1 Interaction
  ;;[1 1 1] Removing Weight
  (bind _asbp_weight_1 (Utilities|Casting|CastToBP_Weight1 OtherActor))
  (bind _output_get (Variables|Default|SetcurrentWeight1 (- (Variables|Default|GetcurrentWeight1) (Variables|/Game/Blueprints/Weights/BP_Weight1.BP_Weight1_C|GetWeigh _asbp_weight_1))))
  (Default|Decrease (Variables|Default|GetCounter%201) _output_get)
  (CallFunction|CheckResult))

(event OnComponentBeginOverlap(Box2)
  (params (OverlappedComponent :type Primitive%20Component%20Object%20Reference) (OtherActor :type Actor%20Object%20Reference) (OtherComp :type Primitive%20Component%20Object%20Reference) (OtherBodyIndex :type Integer) (bFromSweep :type Boolean) (SweepResult :type Hit%20Result%20Structure%20%28by%20ref%29))
  ;[1 1 1] Scale 2 Interaction
  ;;[1 1 1] Adding Weight
  (bind _asbp_weight_1 (Utilities|Casting|CastToBP_Weight1 OtherActor))
  (bind _output_get (Variables|Default|SetCurrentWeight2 (+ (Variables|Default|GetCurrentWeight2) (Variables|/Game/Blueprints/Weights/BP_Weight1.BP_Weight1_C|GetWeigh _asbp_weight_1))))
  (Default|Increase (Variables|Default|GetCounter%202) _output_get)
  (CallFunction|CheckResult))

(event OnComponentEndOverlap(Box2)
  (params (OverlappedComponent :type Primitive%20Component%20Object%20Reference) (OtherActor :type Actor%20Object%20Reference) (OtherComp :type Primitive%20Component%20Object%20Reference) (OtherBodyIndex :type Integer))
  ;[1 1 1] Scale 2 Interaction
  ;;[1 1 1] Removing Weight
  (bind _asbp_weight_1 (Utilities|Casting|CastToBP_Weight1 OtherActor))
  (bind _output_get (Variables|Default|SetCurrentWeight2 (- (Variables|Default|GetCurrentWeight2) (Variables|/Game/Blueprints/Weights/BP_Weight1.BP_Weight1_C|GetWeigh _asbp_weight_1))))
  (Default|Decrease (Variables|Default|GetCounter%202) _output_get)
  (CallFunction|CheckResult))

(event OnComponentBeginOverlap(Box)
  (params (OverlappedComponent :type Primitive%20Component%20Object%20Reference) (OtherActor :type Actor%20Object%20Reference) (OtherComp :type Primitive%20Component%20Object%20Reference) (OtherBodyIndex :type Integer) (bFromSweep :type Boolean) (SweepResult :type Hit%20Result%20Structure%20%28by%20ref%29))
  ;[1 1 1] Scale 1 Interaction
  ;;[1 1 1] Adding Weight
  (bind _asbp_weight_1 (Utilities|Casting|CastToBP_Weight1 OtherActor))
  (bind _output_get (Variables|Default|SetCurrentWeight1 (+ (Variables|/Game/Blueprints/Weights/BP_Weight1.BP_Weight1_C|GetWeigh _asbp_weight_1) (Variables|Default|GetCurrentWeight1))))
  (Default|Increase (Variables|Default|GetCounter%201) _output_get)
  (CallFunction|CheckResult))

(event Custom|CheckResult
  (bind _pilar1 (Variables|Default|GetPilar1))
  (bind _pilar2 (Variables|Default|GetPilar2))
  (bind _relativelocation (Variables|/Script/Engine.SceneComponent|GetRelativeLocation _pilar1))
  (bind _relativelocation_2 (Variables|/Script/Engine.SceneComponent|GetRelativeLocation _pilar2))
  (if (== (Variables|Default|GetCurrentWeight1) (Variables|Default|GetCurrentWeight2))
    (Utilities|FlowControl|Sequence
      (:then_0
        (bind _centerpilar1 (Timeline|Timeline Play)
          (:Update
            (Transformation|SetRelativeLocation _pilar1 (Math|Vector|MakeVector (.x _relativelocation) (.y _relativelocation) _centerpilar1) false false))
          (:Finished
            (Audio|PlaySound2D "/Game/Assets/Sounds/DoorLocked.DoorLocked" 1.0 1.0 0.0 0 0)
            (bind _returnvalue (Actor|GetActorOfClass "/Game/Blueprints/DoorBlueprint/BP_DoorWeight.BP_DoorWeight_C"))
            (Variables|/Game/Blueprints/DoorBlueprint/BP_DoorWeight.BP_DoorWeight_C|SetWeightPuzzle _returnvalue true))))
      (:then_1
        (bind _centerpilar2 (Timeline|Timeline_0 Play)
          (:Update
            (Transformation|SetRelativeLocation _pilar2 (Math|Vector|MakeVector (.x _relativelocation_2) (.y _relativelocation_2) _centerpilar2) false false)))))))

(event EventBeginPlay
  (bind _asbp_weight_counter (Utilities|Casting|CastToBP_WeightCounter (Variables|/Script/Engine.ChildActorComponent|GetChildActor (Variables|Default|GetWeightOfPilar1))))
  (bind _output_get (Variables|Default|SetCounter%201 _asbp_weight_counter))
  (Default|Increase _output_get (Variables|Default|GetCurrentWeight1))
  (bind _asbp_weight_counter_2 (Utilities|Casting|CastToBP_WeightCounter (Variables|/Script/Engine.ChildActorComponent|GetChildActor (Variables|Default|GetWeightOfPilar2))))
  (bind _output_get_2 (Variables|Default|SetCounter%202 _asbp_weight_counter_2))
  (Default|Increase _output_get_2 (Variables|Default|GetCurrentWeight2)))

(fn ConstructionScript)

(fn CalculoVectorBowl2Up)