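; BP_GearButton is a push button for the gear (Engrajes) puzzle, with a separate event that resets the gears.
; Pressed plays a sound and a Timeline that slides the button mesh along Y, then reverses it, using IsPressed to block re-triggering and Loop to end the cycle.
; ResetEngajes finds one actor of each gear class and the puzzle actor via GetActorOfClass, calling each one's reset event in sequence.
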(event Custom|Pressed
  (if (not (Variables|Default|GetIsPressed))
    (Audio|PlaySoundatLocation "/Game/Assets/Sounds/PreassurePlateMove.PreassurePlateMove" (Variables|/Script/Engine.SceneComponent|GetRelativeLocation (Variables|Default|GetAssets2_LocationObject3)) "0, 0, 0" 1.0 1.0 0.0 0 0 0 0)
    (bind _push (Timeline|Timeline Play)
      (:Update
        (Transformation|SetRelativeLocation (Variables|Default|GetAssets2_LocationObject3) (Math|Vector|MakeVector 0.0 (Math|Float|Lerp 0.0 -1.5 _push) 0.0) false false)
        (Variables|Default|SetIsPressed true))
      (:Finished
        (if (Variables|Default|GetLoop)
          (Variables|Default|SetLoop false)
          (Audio|PlaySoundatLocation "/Game/Assets/Sounds/PreassurePlateMove.PreassurePlateMove" (Variables|/Script/Engine.SceneComponent|GetRelativeLocation (Variables|Default|GetAssets2_LocationObject3)) "0, 0, 0" 1.0 1.0 0.0 0 0 0 0)
          (Timeline|Timeline Reverse)
          (else
            (Variables|Default|SetLoop true)
            (Variables|Default|SetIsPressed false)))))))

(event Custom|ResetEngajes
  (Utilities|FlowControl|Sequence
    (:then_0
      (bind _returnvalue (Actor|GetActorOfClass "/Game/Blueprints/Engrajes/BP_Engrajes.BP_Engrajes_C"))
      (Default|Reset _returnvalue))
    (:then_1
      (bind _returnvalue_2 (Actor|GetActorOfClass "/Game/Blueprints/Engrajes/CBP_Engrajes1.CBP_Engrajes1_C"))
      (Default|Reset1 _returnvalue_2))
    (:then_2
      (bind _returnvalue_3 (Actor|GetActorOfClass "/Game/Blueprints/Engrajes/CBP_Engrajes2.CBP_Engrajes2_C"))
      (Default|Reset2 _returnvalue_3))
    (:then_3
      (bind _returnvalue_4 (Actor|GetActorOfClass "/Game/Blueprints/Engrajes/CBP_Engrajes3.CBP_Engrajes3_C"))
      (Default|Reset3 _returnvalue_4))
    (:then_4
      (bind _returnvalue_5 (Actor|GetActorOfClass "/Game/Blueprints/Engrajes/CBP_Engrajes4.CBP_Engrajes4_C"))
      (Default|Reset4 _returnvalue_5))
    (:then_5
      (bind _returnvalue_6 (Actor|GetActorOfClass "/Game/Blueprints/Engrajes/CBP_EngrajesJuan.CBP_EngrajesJuan_C"))
      (Default|Reset5 _returnvalue_6))
    (:then_6
      (bind _returnvalue_7 (Actor|GetActorOfClass "/Game/Blueprints/Engrajes/BP_EngrajesPuzzle.BP_EngrajesPuzzle_C"))
      (Default|ResetCollitin _returnvalue_7))))

(fn ConstructionScript)