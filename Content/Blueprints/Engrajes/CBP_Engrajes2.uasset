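; Gear actor Blueprint with a resettable, physics-driven gear component, Engranaje11.
; BeginPlay caches the actor's starting location in InicialVector.
; The Reset2 event re-enables gravity, collision and physics simulation on the gear, then moves it back to that stored location without sweeping.
; The construction script only calls its parent.
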(event Custom|Reset2
  (bind _engranaje_1__1_ (Variables|Default|GetEngranaje_1__1_))
  (Physics|SetEnableGravity _engranaje_1__1_ true)
  (Collision|SetCollisionEnabled _engranaje_1__1_ "QueryAndPhysics")
  (Physics|SetSimulatePhysics _engranaje_1__1_ true)
  (Transformation|SetWorldLocation _engranaje_1__1_ (Variables|Default|GetInicialVector) false false))

(event EventBeginPlay
  (Variables|Default|SetInicialVector (Transformation|GetActorLocation)))

(fn ConstructionScript
  (|CallParentFunction))