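; Wall gear puzzle in which gears are placed into six slots, and the correct order unlocks BP_DoorGear.
; Each box overlap stores the gear's ID, snaps it to the wall with physics off, disables that slot and runs CheckPuzzle.
; A correct order, with the two end gears interchangeable, plays a timeline that spins gears in alternating directions and sets the door's GearPuzzle flag.
; ResetCollitin re-enables slot collision and clears all stored IDs except the fourth.
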(event OnComponentBeginOverlap(Box)
  (params (OverlappedComponent :type Primitive%20Component%20Object%20Reference) (OtherActor :type Actor%20Object%20Reference) (OtherComp :type Primitive%20Component%20Object%20Reference) (OtherBodyIndex :type Integer) (bFromSweep :type Boolean) (SweepResult :type Hit%20Result%20Structure%20%28by%20ref%29))
  (bind _box (Variables|Default|GetBox))
  (bind _asbp_engrajes (Utilities|Casting|CastToBP_Engrajes OtherActor))
  (Variables|Default|SetIDFirstSlot (Variables|/Game/Blueprints/Engrajes/BP_Engrajes.BP_Engrajes_C|GetID _asbp_engrajes))
  (CallFunction|GettoWall _asbp_engrajes (Transformation|GetWorldLocation _box))
  (Collision|SetCollisionEnabled _box "NoCollision")
  (CallFunction|CheckPuzzle))

(event OnComponentBeginOverlap(Box1)
  (params (OverlappedComponent :type Primitive%20Component%20Object%20Reference) (OtherActor :type Actor%20Object%20Reference) (OtherComp :type Primitive%20Component%20Object%20Reference) (OtherBodyIndex :type Integer) (bFromSweep :type Boolean) (SweepResult :type Hit%20Result%20Structure%20%28by%20ref%29))
  (bind _box1 (Variables|Default|GetBox1))
  (bind _asbp_engrajes (Utilities|Casting|CastToBP_Engrajes OtherActor))
  (Variables|Default|SetIDFirstSlot1 (Variables|/Game/Blueprints/Engrajes/BP_Engrajes.BP_Engrajes_C|GetID _asbp_engrajes))
  (CallFunction|GettoWall _asbp_engrajes (Transformation|GetWorldLocation _box1))
  (Collision|SetCollisionEnabled _box1 "NoCollision")
  (CallFunction|CheckPuzzle))

(event OnComponentBeginOverlap(Box2)
  (params (OverlappedComponent :type Primitive%20Component%20Object%20Reference) (OtherActor :type Actor%20Object%20Reference) (OtherComp :type Primitive%20Component%20Object%20Reference) (OtherBodyIndex :type Integer) (bFromSweep :type Boolean) (SweepResult :type Hit%20Result%20Structure%20%28by%20ref%29))
  (bind _box2 (Variables|Default|GetBox2))
  (bind _asbp_engrajes (Utilities|Casting|CastToBP_Engrajes OtherActor))
  (Variables|Default|SetIDFirstSlot2 (Variables|/Game/Blueprints/Engrajes/BP_Engrajes.BP_Engrajes_C|GetID _asbp_engrajes))
  (CallFunction|GettoWall _asbp_engrajes (Transformation|GetWorldLocation _box2))
  (Collision|SetCollisionEnabled _box2 "NoCollision")
  (CallFunction|CheckPuzzle))

(event OnComponentBeginOverlap(Box3)
  (params (OverlappedComponent :type Primitive%20Component%20Object%20Reference) (OtherActor :type Actor%20Object%20Reference) (OtherComp :type Primitive%20Component%20Object%20Reference) (OtherBodyIndex :type Integer) (bFromSweep :type Boolean) (SweepResult :type Hit%20Result%20Structure%20%28by%20ref%29))
  (bind _box3 (Variables|Default|GetBox3))
  (bind _asbp_engrajes (Utilities|Casting|CastToBP_Engrajes OtherActor))
  (Variables|Default|SetIDFirstSlot3 (Variables|/Game/Blueprints/Engrajes/BP_Engrajes.BP_Engrajes_C|GetID _asbp_engrajes))
  (CallFunction|GettoWall _asbp_engrajes (Transformation|GetWorldLocation _box3))
  (Collision|SetCollisionEnabled _box3 "NoCollision")
  (CallFunction|CheckPuzzle))

(event OnComponentBeginOverlap(Box4)
  (params (OverlappedComponent :type Primitive%20Component%20Object%20Reference) (OtherActor :type Actor%20Object%20Reference) (OtherComp :type Primitive%20Component%20Object%20Reference) (OtherBodyIndex :type Integer) (bFromSweep :type Boolean) (SweepResult :type Hit%20Result%20Structure%20%28by%20ref%29))
  (bind _box4 (Variables|Default|GetBox4))
  (bind _asbp_engrajes (Utilities|Casting|CastToBP_Engrajes OtherActor))
  (Variables|Default|SetIDFirstSlot4 (Variables|/Game/Blueprints/Engrajes/BP_Engrajes.BP_Engrajes_C|GetID _asbp_engrajes))
  (CallFunction|GettoWall _asbp_engrajes (Transformation|GetWorldLocation _box4))
  (Collision|SetCollisionEnabled _box4 "NoCollision")
  (CallFunction|CheckPuzzle))

(event OnComponentBeginOverlap(Box5)
  (params (OverlappedComponent :type Primitive%20Component%20Object%20Reference) (OtherActor :type Actor%20Object%20Reference) (OtherComp :type Primitive%20Component%20Object%20Reference) (OtherBodyIndex :type Integer) (bFromSweep :type Boolean) (SweepResult :type Hit%20Result%20Structure%20%28by%20ref%29))
  (bind _box5 (Variables|Default|GetBox5))
  (bind _asbp_engrajes (Utilities|Casting|CastToBP_Engrajes OtherActor))
  (Variables|Default|SetIDFirstSlot5 (Variables|/Game/Blueprints/Engrajes/BP_Engrajes.BP_Engrajes_C|GetID _asbp_engrajes))
  (CallFunction|GettoWall _asbp_engrajes (Transformation|GetWorldLocation _box5))
  (Collision|SetCollisionEnabled _box5 "NoCollision")
  (CallFunction|CheckPuzzle))

(event Custom|ResetCollitin
  (Utilities|FlowControl|Sequence
    (:then_0
      (Collision|SetCollisionEnabled (Variables|Default|GetBox) "QueryAndPhysics"))
    (:then_1
      (Collision|SetCollisionEnabled (Variables|Default|GetBox1) "QueryAndPhysics"))
    (:then_2
      (Collision|SetCollisionEnabled (Variables|Default|GetBox2) "QueryAndPhysics"))
    (:then_3
      (Collision|SetCollisionEnabled (Variables|Default|GetBox3) "QueryAndPhysics"))
    (:then_4
      (Collision|SetCollisionEnabled (Variables|Default|GetBox4) "QueryAndPhysics"))
    (:then_5
      (Collision|SetCollisionEnabled (Variables|Default|GetBox5) "QueryAndPhysics"))
    (:then_6
      (Variables|Default|SetIDFirstSlot 0)
      (Variables|Default|SetIDFirstSlot1 0)
      (Variables|Default|SetIDFirstSlot2 0)
      (Variables|Default|SetIDFirstSlot4 0)
      (Variables|Default|SetIDFirstSlot5 0))))

(event Custom|StartRotating
  (if (Variables|Default|GetRotate?)
    (Audio|PlaySoundatLocation "/Game/Assets/Sounds/Engranajes_funcionando.Engranajes_funcionando" (Variables|/Script/Engine.SceneComponent|GetRelativeLocation (Variables|Default|GetPared_Engranajes)) "0, 0, 0" 1.0 1.0 0.0 0 0 0 0)
    (bind _newtrack_0 (Timeline|Timeline PlayFromStart)
      (:Update
        (CallFunction|RotateEngrajes _newtrack_0 (stale OnComponentBeginOverlap(Box) _asbp_engrajes) (stale OnComponentBeginOverlap(Box1) _asbp_engrajes) (stale OnComponentBeginOverlap(Box2) _asbp_engrajes) (stale OnComponentBeginOverlap(Box3) _asbp_engrajes) (stale OnComponentBeginOverlap(Box4) _asbp_engrajes) (stale OnComponentBeginOverlap(Box5) _asbp_engrajes))
        (bind _returnvalue (Actor|GetActorOfClass "/Game/Blueprints/DoorBlueprint/BP_DoorGear.BP_DoorGear_C"))
        (Variables|/Game/Blueprints/DoorBlueprint/BP_DoorGear.BP_DoorGear_C|SetGearPuzzle _returnvalue true))
      (:Finished
        (Audio|PlaySound2D "/Game/Assets/Sounds/DoorLocked.DoorLocked" 1.0 1.0 0.0 0 0)))))

(fn ConstructionScript)

(fn GettoWall
  (params (Target :type BP%20Engrajes%20Object%20Reference) (BoxTransform :type Vector))
  (bind _engranaje_1__1_ (Variables|/Game/Blueprints/Engrajes/BP_Engrajes.BP_Engrajes_C|GetEngranaje_1__1_ Target))
  (Physics|SetEnableGravity _engranaje_1__1_ false)
  (Physics|SetSimulatePhysics _engranaje_1__1_ false)
  (Collision|SetCollisionEnabled _engranaje_1__1_ "NoCollision")
  (Variables|Default|SetInWall true)
  (Transformation|SetWorldLocationAndRotation _engranaje_1__1_ (Math|Vector|MakeVector (.x BoxTransform) (.y BoxTransform) (.z BoxTransform)) (Variables|Default|GetEngrajeRotation) false false)
  (CallFunction|StartRotating))

(fn CheckPuzzle
  (if (== (Variables|Default|GetIDFirstSlot) 1)
    (if (== (Variables|Default|GetIDFirstSlot1) 2) :!label _label
      (if (== (Variables|Default|GetIDFirstSlot2) 3)
        (if (== (Variables|Default|GetIDFirstSlot3) 4)
          (if (== (Variables|Default|GetIDFirstSlot4) 5)
            (if (== (Variables|Default|GetIDFirstSlot5) 6)
              (Variables|Default|SetRotate? true :!label _label_2)
              (CallFunction|StartRotating)
              (elif (== (Variables|Default|GetIDFirstSlot5) 1)
                (goto _label_2)))))))
    (elif (== (Variables|Default|GetIDFirstSlot) 6)
      (goto _label))))

(fn RotateEngrajes
  (params (Time :type Float%20%28double-precision%29) (Engraje :type BP%20Engrajes%20Object%20Reference) (Engraje1 :type BP%20Engrajes%20Object%20Reference) (Engraje2 :type BP%20Engrajes%20Object%20Reference) (Engraje3 :type BP%20Engrajes%20Object%20Reference) (Engraje4 :type BP%20Engrajes%20Object%20Reference) (Engraje5 :type BP%20Engrajes%20Object%20Reference))
  (bind _engranaje_1__1_ (Variables|/Game/Blueprints/Engrajes/BP_Engrajes.BP_Engrajes_C|GetEngranaje_1__1_ Engraje1))
  (bind _engranaje_1__1__2 (Variables|/Game/Blueprints/Engrajes/BP_Engrajes.BP_Engrajes_C|GetEngranaje_1__1_ Engraje2))
  (bind _engranaje_1__1__3 (Variables|/Game/Blueprints/Engrajes/BP_Engrajes.BP_Engrajes_C|GetEngranaje_1__1_ Engraje3))
  (bind _engranaje_1__1__4 (Variables|/Game/Blueprints/Engrajes/BP_Engrajes.BP_Engrajes_C|GetEngranaje_1__1_ Engraje4))
  (bind _engranaje_1__1__5 (Variables|/Game/Blueprints/Engrajes/BP_Engrajes.BP_Engrajes_C|GetEngranaje_1__1_ Engraje5))
  (bind _engranaje_1__1__6 (Variables|/Game/Blueprints/Engrajes/BP_Engrajes.BP_Engrajes_C|GetEngranaje_1__1_ Engraje))
  (bind _returnvalue (Transformation|GetWorldRotation _engranaje_1__1__5))
  (bind _returnvalue_2 (Transformation|GetWorldRotation _engranaje_1__1_))
  (bind _returnvalue_3 (Transformation|GetWorldRotation _engranaje_1__1__2))
  (bind _returnvalue_4 (Transformation|GetWorldRotation _engranaje_1__1__3))
  (bind _returnvalue_5 (Transformation|GetWorldRotation _engranaje_1__1__4))
  (bind _returnvalue_6 (Transformation|GetWorldRotation _engranaje_1__1__6))
  (Utilities|FlowControl|Sequence
    (:then_0
      (Transformation|SetWorldRotation _engranaje_1__1__6 (Math|Rotator|MakeRotator (+ (.roll _returnvalue_6) 1.0) (.pitch _returnvalue_6) (.yaw _returnvalue_6)) false false))
    (:then_1
      (Transformation|SetWorldRotation _engranaje_1__1_ (Math|Rotator|MakeRotator (- (.roll _returnvalue_2) 1.0) (.pitch _returnvalue_2) (.yaw _returnvalue_2)) false false))
    (:then_2
      (Transformation|SetWorldRotation _engranaje_1__1__2 (Math|Rotator|MakeRotator (+ (.roll _returnvalue_3) 1.0) (.pitch _returnvalue_3) (.yaw _returnvalue_3)) false false))
    (:then_3
      (Transformation|SetWorldRotation _engranaje_1__1__3 (Math|Rotator|MakeRotator (- (.roll _returnvalue_4) 1.0) (.pitch _returnvalue_4) (.yaw _returnvalue_4)) false false))
    (:then_4
      (Transformation|SetWorldRotation _engranaje_1__1__4 (Math|Rotator|MakeRotator (+ (.roll _returnvalue_5) 1.0) (.pitch _returnvalue_5) (.yaw _returnvalue_5)) false false))
    (:then_5
      (Transformation|SetWorldRotation _engranaje_1__1__5 (Math|Rotator|MakeRotator (- (.roll _returnvalue) 1.0) (.pitch _returnvalue) (.yaw _returnvalue)) false false))))