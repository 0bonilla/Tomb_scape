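; Button Blueprint whose Rotate event turns the R2 piece in 30-degree pitch steps and plays a movement sound.
; A looping six-output MultiGate passes different angles to RotateBrick, but that function ignores them.
; RotateBrick instead advances CurrentAngle by 30, resets it to zero on reaching 360, and applies it as the target's relative pitch.
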(event EventRotate
  (params (Relation :type Integer) (CurrentAngle :type Float%20%28double-precision%29))
  (bind _r2 (Variables|Default|GetR2))
  (Audio|PlaySoundatLocation "/Game/Assets/Sounds/PieceMovement.PieceMovement" (Variables|/Script/Engine.SceneComponent|GetRelativeLocation (Variables|Default|GetR2)) "0, 0, 0" 1.0 1.0 0.0 0 0 0 0)
  (Utilities|FlowControl|MultiGate false true -1
    (:Out%200
      (CallFunction|RotateBrick 3e+01 _r2))
    (:Out%201
      (CallFunction|RotateBrick 6e+01 _r2))
    (:Out%202
      (CallFunction|RotateBrick 9e+01 _r2))
    (:Out%203
      (CallFunction|RotateBrick 1.2e+02 _r2))
    (:Out%204
      (CallFunction|RotateBrick 1.5e+02 _r2))
    (:Out%205
      (CallFunction|RotateBrick 0.0 _r2))))

(fn ConstructionScript)

(fn RotateBrick
  (params (Y%20%28Pitch%29 :type Float%20%28single-precision%29) (Target :type Scene%20Component%20Object%20Reference))
  (if (>= (+ (Variables|Default|GetCurrentAngle) 3e+01) 3.6e+02)
    (Variables|Default|SetCurrentAngle 0.0)
    (else
      (Variables|Default|SetCurrentAngle (+ (Variables|Default|GetCurrentAngle) 3e+01))))
  (Transformation|SetRelativeRotation Target (Math|Rotator|MakeRotator 0.0 (Variables|Default|GetCurrentAngle) 0.0) false false))