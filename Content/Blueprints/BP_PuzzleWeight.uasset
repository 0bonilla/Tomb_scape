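; Balance-scale puzzle that sets WeightPuzzle on BP_DoorWeight and plays a sound when both bowls hold equal weight.
; BP_Weight1 actors entering or leaving either box trigger update that bowl's total.
; Timelines lerp the two pillars in opposite Z directions, offset by that bowl's total rather than the changed weight.
; Each finished timeline checks for equality, so two emptied bowls also count as solved.
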(event OnComponentEndOverlap(Box)
  (params (OverlappedComponent :type Primitive%20Component%20Object%20Reference) (OtherActor :type Actor%20Object%20Reference) (OtherComp :type Primitive%20Component%20Object%20Reference) (OtherBodyIndex :type Integer))
  ;[1 1 1] Scale 1 Interaction
  ;;[1 1 1] Removing Weight
  (bind _asbp_weight_1 (Utilities|Casting|CastToBP_Weight1 OtherActor))
  (CallFunction|CalculoVectorBowl1Up)
  (Variables|Default|SetcurrentWeight1 (- (Variables|Default|GetcurrentWeight1) (Variables|/Game/Blueprints/Weights/BP_Weight1.BP_Weight1_C|GetWeigh _asbp_weight_1)))
  (bind _animationtrack (Timeline|Timeline_0 PlayFromStart)
    (:Update
      (CallFunction|WeightUpBowl1Movement _animationtrack (Variables|Default|GetMoveWeight1))
      (CallFunction|WeightDownBowl2Movement _animationtrack (Variables|Default|GetMoveWeight2)))
    (:Finished
      (CallFunction|CheckResult))))

(event OnComponentBeginOverlap(Box2)
  (params (OverlappedComponent :type Primitive%20Component%20Object%20Reference) (OtherActor :type Actor%20Object%20Reference) (OtherComp :type Primitive%20Component%20Object%20Reference) (OtherBodyIndex :type Integer) (bFromSweep :type Boolean) (SweepResult :type Hit%20Result%20Structure%20%28by%20ref%29))
  ;[1 1 1] Scale 2 Interaction
  ;;[1 1 1] Adding Weight
  (bind _asbp_weight_1 (Utilities|Casting|CastToBP_Weight1 OtherActor))
  (Variables|Default|SetCurrentWeight2 (+ (Variables|Default|GetCurrentWeight2) (Variables|/Game/Blueprints/Weights/BP_Weight1.BP_Weight1_C|GetWeigh _asbp_weight_1)))
  (CallFunction|CalculoVectorBowl2Down)
  (bind _animationtrack (Timeline|Timeline_1 PlayFromStart)
    (:Update
      (CallFunction|WeightUpBowl1Movement _animationtrack (Variables|Default|GetMoveWeight1))
      (CallFunction|WeightDownBowl2Movement _animationtrack (Variables|Default|GetMoveWeight2)))
    (:Finished
      (CallFunction|CheckResult))))

(event OnComponentEndOverlap(Box2)
  (params (OverlappedComponent :type Primitive%20Component%20Object%20Reference) (OtherActor :type Actor%20Object%20Reference) (OtherComp :type Primitive%20Component%20Object%20Reference) (OtherBodyIndex :type Integer))
  ;[1 1 1] Scale 2 Interaction
  ;;[1 1 1] Removing Weight
  (bind _asbp_weight_1 (Utilities|Casting|CastToBP_Weight1 OtherActor))
  (CallFunction|CalculoVectorBowl2Up)
  (Variables|Default|SetCurrentWeight2 (- (Variables|Default|GetCurrentWeight2) (Variables|/Game/Blueprints/Weights/BP_Weight1.BP_Weight1_C|GetWeigh _asbp_weight_1)))
  (bind _animationtrack (Timeline|Timeline_2 PlayFromStart)
    (:Update
      (CallFunction|WeightDownBowl1Movement _animationtrack (Variables|Default|GetMoveWeight1))
      (CallFunction|WeightUpBowl2Movement _animationtrack (Variables|Default|GetMoveWeight2)))
    (:Finished
      (CallFunction|CheckResult))))

(event OnComponentBeginOverlap(Box)
  (params (OverlappedComponent :type Primitive%20Component%20Object%20Reference) (OtherActor :type Actor%20Object%20Reference) (OtherComp :type Primitive%20Component%20Object%20Reference) (OtherBodyIndex :type Integer) (bFromSweep :type Boolean) (SweepResult :type Hit%20Result%20Structure%20%28by%20ref%29))
  ;[1 1 1] Scale 1 Interaction
  ;;[1 1 1] Adding Weight
  (bind _asbp_weight_1 (Utilities|Casting|CastToBP_Weight1 OtherActor))
  (Variables|Default|SetCurrentWeight1 (+ (Variables|/Game/Blueprints/Weights/BP_Weight1.BP_Weight1_C|GetWeigh _asbp_weight_1) (Variables|Default|GetCurrentWeight1)))
  (CallFunction|CalculoVectorBowl1Down)
  (bind _animationtrack (Timeline|Timeline PlayFromStart)
    (:Update
      (CallFunction|WeightDownBowl1Movement _animationtrack (Variables|Default|GetMoveWeight1))
      (CallFunction|WeightUpBowl2Movement _animationtrack (Variables|Default|GetMoveWeight2)))
    (:Finished
      (CallFunction|CheckResult))))

(event Custom|CheckResult
  (if (== (Variables|Default|GetCurrentWeight1) (Variables|Default|GetCurrentWeight2))
    (Audio|PlaySound2D "/Game/Assets/Sounds/DoorLocked.DoorLocked" 1.0 1.0 0.0 0 0)
    (bind _returnvalue (Actor|GetActorOfClass "/Game/Blueprints/DoorBlueprint/BP_DoorWeight.BP_DoorWeight_C"))
    (Variables|/Game/Blueprints/DoorBlueprint/BP_DoorWeight.BP_DoorWeight_C|SetWeightPuzzle _returnvalue true)))

(fn ConstructionScript)

(fn WeightUpBowl1Movement
  (params (Time :type Float%20%28double-precision%29) (Movement :type Vector))
  (bind _pilar1 (Variables|Default|GetPilar1))
  (bind _returnvalue (Transformation|GetWorldLocation _pilar1))
  (Transformation|SetWorldLocation _pilar1 (Math|Vector|MakeVector (.x _returnvalue) (.y _returnvalue) (Math|Float|Lerp (.z _returnvalue) (.z Movement) Time)) false false))

(fn WeightDownBowl1Movement
  (params (Time :type Float%20%28double-precision%29) (Movement :type Vector))
  (bind _pilar1 (Variables|Default|GetPilar1))
  (bind _returnvalue (Transformation|GetWorldLocation _pilar1))
  (Transformation|SetWorldLocation _pilar1 (Math|Vector|MakeVector (.x _returnvalue) (.y _returnvalue) (Math|Float|Lerp (.z _returnvalue) (.z Movement) Time)) false false))

(fn WeightUpBowl2Movement
  (params (Time :type Float%20%28double-precision%29) (Movement :type Vector))
  (bind _pilar2 (Variables|Default|GetPilar2))
  (bind _returnvalue (Transformation|GetWorldLocation _pilar2))
  (Transformation|SetWorldLocation _pilar2 (Math|Vector|MakeVector (.x _returnvalue) (.y _returnvalue) (Math|Float|Lerp (.z _returnvalue) (.z Movement) Time)) false false))

(fn WeightDownBowl2Movement
  (params (Time :type Float%20%28double-precision%29) (Movement :type Vector))
  (bind _pilar2 (Variables|Default|GetPilar2))
  (bind _returnvalue (Transformation|GetWorldLocation _pilar2))
  (Transformation|SetWorldLocation _pilar2 (Math|Vector|MakeVector (.x _returnvalue) (.y _returnvalue) (Math|Float|Lerp (.z _returnvalue) (.z Movement) Time)) false false))

(fn CalculoVectorBowl1Down
  (bind _pilar2 (Variables|Default|GetPilar2))
  (bind _pilar1 (Variables|Default|GetPilar1))
  (bind _returnvalue (Transformation|GetWorldLocation _pilar2))
  (bind _returnvalue_2 (Transformation|GetWorldLocation _pilar1))
  (Variables|Default|SetMoveWeight1 (Math|Vector|MakeVector (.x _returnvalue_2) (.y _returnvalue_2) (- (.z _returnvalue_2) (Variables|Default|GetCurrentWeight1))))
  (Variables|Default|SetMoveWeight2 (Math|Vector|MakeVector (.x _returnvalue) (.y _returnvalue) (+ (.z _returnvalue) (Variables|Default|GetCurrentWeight1)))))

(fn CalculoVectorBowl1Up
  (bind _pilar2 (Variables|Default|GetPilar2))
  (bind _pilar1 (Variables|Default|GetPilar1))
  (bind _returnvalue (Transformation|GetWorldLocation _pilar2))
  (bind _returnvalue_2 (Transformation|GetWorldLocation _pilar1))
  (Variables|Default|SetMoveWeight1 (Math|Vector|MakeVector (.x _returnvalue_2) (.y _returnvalue_2) (+ (Variables|Default|GetCurrentWeight1) (.z _returnvalue_2))))
  (Variables|Default|SetMoveWeight2 (Math|Vector|MakeVector (.x _returnvalue) (.y _returnvalue) (- (.z _returnvalue) (Variables|Default|GetCurrentWeight1)))))

(fn CalculoVectorBowl2Down
  (bind _pilar1 (Variables|Default|GetPilar1))
  (bind _pilar2 (Variables|Default|GetPilar2))
  (bind _returnvalue (Transformation|GetWorldLocation _pilar2))
  (bind _returnvalue_2 (Transformation|GetWorldLocation _pilar1))
  (Variables|Default|SetMoveWeight1 (Math|Vector|MakeVector (.x _returnvalue_2) (.y _returnvalue_2) (+ (Variables|Default|GetCurrentWeight2) (.z _returnvalue_2))))
  (Variables|Default|SetMoveWeight2 (Math|Vector|MakeVector (.x _returnvalue) (.y _returnvalue) (- (.z _returnvalue) (Variables|Default|GetCurrentWeight2)))))

(fn CalculoVectorBowl2Up
  (bind _pilar1 (Variables|Default|GetPilar1))
  (bind _pilar2 (Variables|Default|GetPilar2))
  (bind _returnvalue (Transformation|GetWorldLocation _pilar1))
  (bind _returnvalue_2 (Transformation|GetWorldLocation _pilar2))
  (Variables|Default|SetMoveWeight2 (Math|Vector|MakeVector (.x _returnvalue_2) (.y _returnvalue_2) (+ (Variables|Default|GetCurrentWeight2) (.z _returnvalue_2))))
  (Variables|Default|SetMoveWeight1 (Math|Vector|MakeVector (.x _returnvalue) (.y _returnvalue) (- (.z _returnvalue) (Variables|Default|GetCurrentWeight2)))))